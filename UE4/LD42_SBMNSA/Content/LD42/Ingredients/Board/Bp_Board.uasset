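; Game board that spawns a centered grid of BP_Tile actors and drives the spread of corruption outbreaks.
; BeginPlay sizes the grid from a throwaway tile's bounds, then stores tiles in a coordinate-keyed map and a neutral list.
; An outbreak spawns on a random neutral tile at start and on a looping timer.
; Helpers provide tile, orthogonal-neighbor and random-by-state lookups, and CheckGameOver shows the game-over widget when no neutral tiles remain.
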(event `self.ReceiveBeginPlay`
  (bind (_tileboundextent_x _tileboundextent_y _tileboundextent_z) (`KismetMathLibrary.BreakVector` (`self.TileBoundExtent`)))
  (bind (_tileboundextent_x_2 _tileboundextent_y_2 _tileboundextent_z_2) (`KismetMathLibrary.BreakVector` (`self.TileBoundExtent`)))
  (bind (_tileboundextent_x_3 _tileboundextent_y_3 _tileboundextent_z_3) (`KismetMathLibrary.BreakVector` (`self.TileBoundExtent`)))
  (`|ExecutionSequence`
    (:`then_0`
      ;[1 1 1] Get bounds infos
      (bind _returnvalue (`|SpawnActorFromClass` "/Game/LD42/Ingredients/Board/BP_Tile.BP_Tile_C" (`KismetMathLibrary.MakeTransform` (0.0 0.0 0.0)) "Undefined" "OverrideRootScale" null (struct) null))
      (bind (_origin _boxextent) (`KismetSystemLibrary.GetComponentBounds` (`/Game/LD42/Ingredients/Board/BP_Tile.TileSprite` _returnvalue)))
      (set `self.TileBoundOrigin` _origin)
      (set `self.TileBoundExtent` _boxextent)
      (`self.K2_DestroyActor` _returnvalue))
    (:`then_1`
      ;[1 1 1] Set Offset to recenter Tiles on screen
      (set `self.TileOffsetForRecenter` (`KismetMathLibrary.MakeVector` (* (`self.ColumnQty`) _tileboundextent_x_3) _tileboundextent_y_3 (* (`self.RowQty`) _tileboundextent_z_3))))
    (:`then_2`
      ;[1 1 1] Create 2D array depending on Columns and Rows / Populate with Tiles / Make Tiles maps with coordinates
      (for _index (range (`self.ColumnQty`))
        (for _index_2 (range (`self.RowQty`))
          (bind _str_tilecoordinates (make `/Game/LD42/Ingredients/Board/STR_TileCoordinates` _index _index_2))
          (bind _returnvalue_2 (`|SpawnActorFromClass` "/Game/LD42/Ingredients/Board/BP_Tile.BP_Tile_C" (`KismetMathLibrary.MakeTransform` (- (`KismetMathLibrary.MakeVector` (* _index (* 2 _tileboundextent_x_2)) 10.0 (* _index_2 (* 2 _tileboundextent_z_2))) (`self.TileOffsetForRecenter`))) "Undefined" "OverrideRootScale" self _str_tilecoordinates null))
          (`BlueprintMapLibrary.Map_Add` (`self.Tiles`) _str_tilecoordinates _returnvalue_2)
          (`KismetArrayLibrary.Array_Add` (`self.NeutralTiles`) _returnvalue_2))))
    (:`then_3`
      ;[1 1 1] Determine max X and Z distances
      (set `self.XMaxDistance` (* (`self.ColumnQty`) _tileboundextent_x))
      (set `self.ZMaxDistance` (* (`self.RowQty`) _tileboundextent_z)))
    (:`then_4`
      (`KismetSystemLibrary.K2_SetTimerDelegate` (delegate `CustomEvent_0`) (`self.NewOutbreakTimer`) true)
      (`self.CreateNewOutbreak` :!label _label))))

(event `CustomEvent_0`
  (goto _label))

(fn `CheckGameOver`
  (if (== (`KismetArrayLibrary.Array_Length` (`self.NeutralTiles`)) 0)
    (bind _returnvalue (`|CreateWidget` "/Game/LD42/Menu/WBP_GameOver.WBP_GameOver_C"))
    (`UserWidget.AddToViewport` _returnvalue 0)))

(fn `CreateNewOutbreak`
  (locals (Local_RandomTile :type "/Game/LD42/Ingredients/Board/BP_Tile Object Reference"))
  (set `local.Local_RandomTile` (`self.GetRandomTile` true "NewEnumerator0"))
  (`|SpawnActorFromClass` "/Game/LD42/Ingredients/Infection/BP_Outbreak.BP_Outbreak_C" (`self.GetTransform` (`local.Local_RandomTile`)) "Undefined" "OverrideRootScale" null (`|MakeArray` (`local.Local_RandomTile`)) null))

(fn `GetAdjacentTiles`
  (params (Coordinates :type "/Game/LD42/Ingredients/Board/STR_TileCoordinates Structure"))
  (returns (AdjacentTiles :type "Array of /Game/LD42/Ingredients/Board/BP_Tile Object Reference"))
  (locals (Local_Tiles :type "Array of /Game/LD42/Ingredients/Board/BP_Tile Object Reference"))
  (bind (_coordinates_x _coordinates_z) (break `/Game/LD42/Ingredients/Board/STR_TileCoordinates` (`local.Coordinates`)))
  (bind (_coordinates_x_2 _coordinates_z_2) (break `/Game/LD42/Ingredients/Board/STR_TileCoordinates` (`local.Coordinates`)))
  (bind (_coordinates_x_3 _coordinates_z_3) (break `/Game/LD42/Ingredients/Board/STR_TileCoordinates` (`local.Coordinates`)))
  (bind (_coordinates_x_4 _coordinates_z_4) (break `/Game/LD42/Ingredients/Board/STR_TileCoordinates` (`local.Coordinates`)))
  (bind _returnvalue (- _coordinates_x_4 1))
  (bind _returnvalue_2 (- _coordinates_z_2 1))
  (bind _returnvalue_3 (+ _coordinates_x 1))
  (bind _returnvalue_4 (+ _coordinates_z_3 1))
  (`|ExecutionSequence`
    (:`then_0`
      ;[1 1 1] Left
      (if (>= _returnvalue 0)
        (`KismetArrayLibrary.Array_Add` (`local.Local_Tiles`) (`self.GetTile` (make `/Game/LD42/Ingredients/Board/STR_TileCoordinates` _returnvalue _coordinates_z_4)))))
    (:`then_1`
      ;[1 1 1] Right
      (if (< _returnvalue_3 (`self.ColumnQty`))
        (`KismetArrayLibrary.Array_Add` (`local.Local_Tiles`) (`self.GetTile` (make `/Game/LD42/Ingredients/Board/STR_TileCoordinates` _returnvalue_3 _coordinates_z)))))
    (:`then_2`
      ;[1 1 1] Down
      (if (>= _returnvalue_2 0)
        (`KismetArrayLibrary.Array_Add` (`local.Local_Tiles`) (`self.GetTile` (make `/Game/LD42/Ingredients/Board/STR_TileCoordinates` _coordinates_x_2 _returnvalue_2)))))
    (:`then_3`
      ;[1 1 1] Up
      (if (< _returnvalue_4 (`self.RowQty`))
        (`KismetArrayLibrary.Array_Add` (`local.Local_Tiles`) (`self.GetTile` (make `/Game/LD42/Ingredients/Board/STR_TileCoordinates` _coordinates_x_3 _returnvalue_4)))))
    (:`then_4`
      (return (`local.Local_Tiles`)))))

(fn `GetRandomTile`
  (params (SpecificState :type Boolean) (State :type "/Game/LD42/Ingredients/Board/EN_TileState Enum" :default "NewEnumerator0"))
  (returns (Tile :type "/Game/LD42/Ingredients/Board/BP_Tile Object Reference"))
  (locals (RandomX :type Integer) (RandomZ :type Integer))
  (bind _corruptedtiles (`self.CorruptedTiles`))
  (bind _tiles (`self.Tiles`))
  (bind _neutraltiles (`self.NeutralTiles`))
  (if SpecificState
    ;[1 1 1] Specific state
    (switch `/Game/LD42/Ingredients/Board/EN_TileState` (`local.State`)
      (:`NewEnumerator0`
        (return (`|GetArrayItem` _neutraltiles (`KismetMathLibrary.RandomInteger` (- (`KismetArrayLibrary.Array_Length` _neutraltiles) 1)))))
      (:`NewEnumerator1`
        (return (`|GetArrayItem` _corruptedtiles (`KismetMathLibrary.RandomInteger` (- (`KismetArrayLibrary.Array_Length` _corruptedtiles) 1))))))
    (else
      ;[1 1 1] All tiles
      (bind _values (`BlueprintMapLibrary.Map_Values` _tiles))
      (return (`|GetArrayItem` _values (`KismetMathLibrary.RandomInteger` (- (`BlueprintMapLibrary.Map_Length` _tiles) 1)))))))

(fn `GetTile`
  (params (Coordinates :type "/Game/LD42/Ingredients/Board/STR_TileCoordinates Structure"))
  (returns (Tile :type "/Game/LD42/Ingredients/Board/BP_Tile Object Reference"))
  (bind (_value _returnvalue) (`BlueprintMapLibrary.Map_Find` (`self.Tiles`) Coordinates))
  (if _returnvalue
    (return _value)
    (else
      (return null))))

(fn `UserConstructionScript`)