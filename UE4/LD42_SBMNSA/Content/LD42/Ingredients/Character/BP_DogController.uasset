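; BP_DogController is the input controller that moves the player's dog pawn in the X-Z plane.
; The MoveRight and MoveUp axis events cast player pawn 0 to BP_DogPawn and offset its world position along X and Z respectively.
; Each offset is the axis value times DogSpeed, with no delta-time scaling, so movement speed depends on frame rate.
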(event `InputAxis|MoveRight`
  (params (AxisValue :type "Float (single-precision)"))
  (bind _asbp_dog_pawn (cast `/Game/LD42/Ingredients/Character/BP_DogPawn` (`GameplayStatics.GetPlayerPawn` 0)))
  (`self.K2_AddActorWorldOffset` _asbp_dog_pawn (`KismetMathLibrary.MakeVector` (* AxisValue (`self.DogSpeed`))) false false))

(event `InputAxis|MoveUp`
  (params (AxisValue :type "Float (single-precision)"))
  (bind _asbp_dog_pawn (cast `/Game/LD42/Ingredients/Character/BP_DogPawn` (`GameplayStatics.GetPlayerPawn` 0)))
  (`self.K2_AddActorWorldOffset` _asbp_dog_pawn (`KismetMathLibrary.MakeVector` 0.0 0.0 (* AxisValue (`self.DogSpeed`))) false false))

(fn `UserConstructionScript`)