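; Player-controlled 2D dog pawn that moves on the board's X/Z plane, dodging projectiles and barking to clean corrupted tiles.
; AZERTY or QWERTY axes, chosen by a GameInstance flag polled on Tick, share bounds-clamped movement that changes speed over corruption.
; Bark needs enough BP_BarkReserve resource and resets tiles within BarkRange.
; Projectile hits update that reserve, and both actions briefly swap the sprite via retriggerable delays.
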(event `self.ReceiveBeginPlay`
  (`|ExecutionSequence`
    (:`then_0`
      (`self.EnableInput` (`GameplayStatics.GetPlayerController` 0)))
    (:`then_1`
      (bind _outactors (`GameplayStatics.GetAllActorsOfClass` "/Game/LD42/Ingredients/Ressource/BP_BarkReserve.BP_BarkReserve_C"))
      (set `self.BarkReserve` (`|GetArrayItem` _outactors)))))

(event `InputAxis|MoveRightAzerty`
  (params (AxisValue :type "Float (single-precision)"))
  (bind _returnvalue_x (`KismetMathLibrary.BreakVector` (`self.K2_GetActorLocation`)))
  (bind (_origin _boxextent) (`KismetSystemLibrary.GetComponentBounds` (`self.PaperSprite`)))
  (bind _xmaxdistance (`/Game/LD42/Ingredients/Board/Bp_Board.XMaxDistance` (`/Game/LD42/Ingredients/BP_FunctionLibrary.GetBoard`)))
  ;[1 1 1] Move X Axis
  (if (`self.AzertyActive`)
    (bind _asbp_dog_pawn (cast `/Game/LD42/Ingredients/Character/BP_DogPawn` (`GameplayStatics.GetPlayerPawn` 0) :!label _label))
    (bind _returnvalue (* (select `bool` (`self.AzertyActive`) :`false` (`KismetMathLibrary.FClamp` (stale `InputAxis|MoveRightQuerty` AxisValue) -1.0) :`true` (`KismetMathLibrary.FClamp` AxisValue -1.0)) (select `bool` (`self.InCorruption`) :`false` (`self.DogSpeed`) :`true` (* (`self.DogSpeed`) (`self.DogCorruptionSpeedRatio`)))))
    (bind _returnvalue_2 (+ _returnvalue _returnvalue_x))
    (if (and (<= _returnvalue_2 (- _xmaxdistance (.x _boxextent))) (>= _returnvalue_2 (+ (- 0.0 _xmaxdistance) (.x _boxextent))))
      (`self.K2_AddActorWorldOffset` _asbp_dog_pawn (`KismetMathLibrary.MakeVector` _returnvalue) false false))))

(event `InputAxis|MoveRightQuerty`
  (params (AxisValue :type "Float (single-precision)"))
  ;[1 1 1] Move X Axis
  (if (not (`self.AzertyActive`))
    (goto _label)))

(event `InputAction|Bark`
  (params (Key :type "Key Structure"))
  (bind _barkreserve (`self.BarkReserve`))
  (:`Pressed`
    (if (>= (`KismetArrayLibrary.Array_LastIndex` (`/Game/LD42/Ingredients/Ressource/BP_BarkReserve.BarkRessource` _barkreserve)) 9)
      (`/Game/LD42/Ingredients/Ressource/BP_BarkReserve.UseBark` _barkreserve)
      (`self.BarkEffect`)
      (`PaperSpriteComponent.SetSprite` (`self.PaperSprite`) "/Game/LD42/Ingredients/Character/SPT_MainCharacter_Bark.SPT_MainCharacter_Bark")
      (`KismetSystemLibrary.RetriggerableDelay` 0.5)
      (`PaperSpriteComponent.SetSprite` (`self.PaperSprite`) "/Game/LD42/Ingredients/Character/SPT_MainCharacter.SPT_MainCharacter"))))

(event `InputAxis|MoveUpAzerty`
  (params (AxisValue :type "Float (single-precision)"))
  (bind (_returnvalue_x _returnvalue_y _returnvalue_z) (`KismetMathLibrary.BreakVector` (`self.K2_GetActorLocation`)))
  (bind (_origin _boxextent) (`KismetSystemLibrary.GetComponentBounds` (`self.PaperSprite`)))
  (bind _zmaxdistance (`/Game/LD42/Ingredients/Board/Bp_Board.ZMaxDistance` (`/Game/LD42/Ingredients/BP_FunctionLibrary.GetBoard`)))
  (if (`self.AzertyActive`)
    ;[1 1 1] Move Z Axis
    (bind _asbp_dog_pawn (cast `/Game/LD42/Ingredients/Character/BP_DogPawn` (`GameplayStatics.GetPlayerPawn` 0) :!label _label_2))
    (bind _returnvalue (* (select `bool` (`self.AzertyActive`) :`false` (`KismetMathLibrary.FClamp` (stale `InputAxis|MoveUpQuerty` AxisValue) -1.0) :`true` (`KismetMathLibrary.FClamp` AxisValue -1.0)) (select `bool` (`self.InCorruption`) :`false` (`self.DogSpeed`) :`true` (* (`self.DogSpeed`) (`self.DogCorruptionSpeedRatio`)))))
    (bind _returnvalue_2 (+ _returnvalue _returnvalue_z))
    (if (and (<= _returnvalue_2 (- _zmaxdistance (.z _boxextent))) (>= _returnvalue_2 (+ (- 0.0 _zmaxdistance) (.z _boxextent))))
      (`self.K2_AddActorWorldOffset` _asbp_dog_pawn (`KismetMathLibrary.MakeVector` 0.0 0.0 _returnvalue) false false))))

(event `self.ProjectileColl.OnComponentBeginOverlap`
  (params (OverlappedComponent :type "PrimitiveComponent Object Reference") (OtherActor :type "Actor Object Reference") (OtherComp :type "PrimitiveComponent Object Reference") (OtherBodyIndex :type Integer) (bFromSweep :type Boolean) (SweepResult :type "HitResult Structure (by ref)"))
  (bind _asbp_projectile (cast `/Game/LD42/Ingredients/Clodo/BP_Projectile` OtherActor))
  (`self.K2_DestroyActor` _asbp_projectile)
  (`/Game/LD42/Ingredients/Ressource/BP_BarkReserve.TakeDamage_Update` (`self.BarkReserve`))
  (`PaperSpriteComponent.SetSprite` (`self.PaperSprite`) "/Game/LD42/Ingredients/Character/SPT_MainCharacter_Hurt.SPT_MainCharacter_Hurt")
  (`KismetSystemLibrary.RetriggerableDelay` 0.5)
  (`PaperSpriteComponent.SetSprite` (`self.PaperSprite`) "/Game/LD42/Ingredients/Character/SPT_MainCharacter.SPT_MainCharacter"))

(event `InputAxis|MoveUpQuerty`
  (params (AxisValue :type "Float (single-precision)"))
  (if (not (`self.AzertyActive`))
    (goto _label_2)))

(event `self.ReceiveTick`
  (params (DeltaSeconds :type "Float (single-precision)"))
  (`|ExecutionSequence`
    (:`then_0`
      (bind _returnvalue (`self.IsInCorruption`))
      (set `self.InCorruption` _returnvalue))
    (:`then_1`
      (bind _asbp_game_instance (cast `/Game/LD42/Ingredients/System/BP_GameInstance` (`GameplayStatics.GetGameInstance`)))
      (set `self.AzertyActive` (`/Game/LD42/Ingredients/System/BP_GameInstance.AzertyActive` _asbp_game_instance)))))

(fn `BarkEffect`
  ;[1 1 1] Clean Tiles
  (for _array_element (`PrimitiveComponent.GetOverlappingActors` (`self.BarkRange`) "/Game/LD42/Ingredients/Board/BP_Tile.BP_Tile_C")
    (bind _asbp_tile (cast `/Game/LD42/Ingredients/Board/BP_Tile` _array_element))
    (if (`|EnumEquality` (`/Game/LD42/Ingredients/Board/BP_Tile.TileState` _asbp_tile) "NewEnumerator1")
      (`/Game/LD42/Ingredients/Board/BP_Tile.ChangeTileState` _asbp_tile "NewEnumerator0"))))

(fn `IsInCorruption`
  (returns (ReturnValue :type Boolean))
  (for _array_element (`PrimitiveComponent.GetOverlappingActors` (`self.CorruptionColl`) "/Game/LD42/Ingredients/Board/BP_Tile.BP_Tile_C")
    (bind _asbp_tile (cast `/Game/LD42/Ingredients/Board/BP_Tile` _array_element))
    (if (`|EnumEquality` (`/Game/LD42/Ingredients/Board/BP_Tile.TileState` _asbp_tile) "NewEnumerator1")
      (return true)))
  (return false))

(fn `UserConstructionScript`)