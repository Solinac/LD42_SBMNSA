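; Projectile actor for the Clodo ingredient that flies from its spawn point toward a targeted player location.
; On BeginPlay a timeline drives a lerp between the two positions and a pitch rotation, whose sign flips when the player is on the right side.
; The target is a stored position rather than a tracked actor, and the projectile destroys itself when the timeline ends, with no hit logic in its graph.
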(event `self.ReceiveBeginPlay`
  (set `self.SpawnLocation` (`self.K2_GetActorLocation` self))
  (bind (_direction _alphalocation _rotation) (`Timeline|Timeline_0`)
    (:`Update`
      (`self.K2_SetActorLocationAndRotation` self (`KismetMathLibrary.VLerp` (`self.SpawnLocation`) (`self.PlayerTargetedLocation`) _alphalocation) (`KismetMathLibrary.MakeRotator` 0.0 (* _rotation (select `bool` (`self.PlayerOnRightSide`) :`false` 1.0 :`true` -1.0 :!type "Float (single-precision)"))) false false))
    (:`Finished`
      (`self.K2_DestroyActor` self))))

(fn `UserConstructionScript`)