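; BP_Clodo is a stationary-looking 2D sprite character that throws a projectile at the player when they come close.
; Each tick it measures XZ-plane distance to the player pawn and, within range, turns angry and spawns a BP_Projectile.
; It passes the projectile the player's position and side, found by comparing distances from itself and a point offset along X.
; A DoOnce gate with delays restores the neutral sprite, then re-arms the attack after a cooldown.
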(event `self.ReceiveTick`
  (params (DeltaSeconds :type "Float (single-precision)"))
  (bind _returnvalue (`self.K2_GetActorLocation` self))
  (bind _returnvalue_2 (`self.K2_GetActorLocation` (`GameplayStatics.GetPlayerPawn` 0)))
  (bind (_returnvalue_x _returnvalue_y _returnvalue_z) (`KismetMathLibrary.BreakVector` (- _returnvalue_2 _returnvalue)))
  (bind (_returnvalue_x_2 _returnvalue_y_2 _returnvalue_z_2) (`KismetMathLibrary.BreakVector` (- _returnvalue_2 (+ _returnvalue (10.0 0.0 0.0)))))
  (bind _returnvalue_3 (`KismetMathLibrary.VSize` (`KismetMathLibrary.MakeVector` _returnvalue_x 0.0 _returnvalue_z)))
  (if (<= _returnvalue_3 60.0)
    (`/Engine/EditorBlueprintResources/StandardMacros.DoOnce` false :!label _label
      (:`Completed`
        (`|ExecutionSequence`
          (:`then_0`
            (`PaperSpriteComponent.SetSprite` (`self.PaperSprite`) "/Game/LD42/Ingredients/Clodo/SPT_Clodo_Angry.SPT_Clodo_Angry")
            (bind _returnvalue_4 (`|SpawnActorFromClass` "/Game/LD42/Ingredients/Clodo/BP_Projectile.BP_Projectile_C" (`self.GetTransform` self) "Undefined" "OverrideRootScale" null null))
            (set `/Game/LD42/Ingredients/Clodo/BP_Projectile.PlayerOnRightSide` (> _returnvalue_3 (`KismetMathLibrary.VSize` (`KismetMathLibrary.MakeVector` _returnvalue_x_2 0.0 _returnvalue_z_2))) _returnvalue_4)
            (set `/Game/LD42/Ingredients/Clodo/BP_Projectile.PlayerTargetedLocation` (`self.K2_GetActorLocation` (`GameplayStatics.GetPlayerPawn` 0)) _returnvalue_4))
          (:`then_1`
            (`KismetSystemLibrary.Delay` 1.0)
            (`PaperSpriteComponent.SetSprite` (`self.PaperSprite`) "/Game/LD42/Ingredients/Clodo/SPT_Clodo_Neutral.SPT_Clodo_Neutral")
            (`KismetSystemLibrary.Delay` 2.0)
            (goto _label :!via `Reset`)))))))

(fn `UserConstructionScript`)