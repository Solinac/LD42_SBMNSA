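; A 2D citizen that wanders the BP_Board play area and rewards the player for coming close.
; Tick moves it in XZ; looping gates randomly re-pick each axis direction at intervals, pausing briefly when an edge hit reverses it.
; When the player comes near, a short delay makes it happy, swapping its sprite and spawning a burst of BP_Ressources via a self-looping DoN.
; It returns to neutral after a timed cooldown.
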(event `RetriggerZSpeedChange`
  (set `self.ZSpeed` (* (`self.ZSpeed`) -1.0))
  (`|ExecutionSequence`
    (:`then_0`
      (goto _label_2 :!via `Close`))
    (:`then_1`
      (`KismetSystemLibrary.Delay` 3.0)
      (`|ExecutionSequence`
        (:`then_0`
          (goto _label_2 :!via `Open`))
        (:`then_1`
          (`KismetSystemLibrary.Delay` (`KismetMathLibrary.RandomFloatInRange` 3.0 10.0) :!label _label)
          (`/Engine/EditorBlueprintResources/StandardMacros.Gate` false :!label _label_2
            (:`Exit`
              (if (`KismetMathLibrary.RandomBool`)
                (set `self.ZSpeed` 10.0)
                (goto _label)
                (else
                  (set `self.ZSpeed` -10.0)
                  (goto _label))))))))))

(event `REtriggerXSpeedChange`
  (set `self.XSpeed` (* (`self.XSpeed`) -1.0))
  (`|ExecutionSequence`
    (:`then_0`
      (goto _label_4 :!via `Close`))
    (:`then_1`
      (`KismetSystemLibrary.Delay` 3.0)
      (`|ExecutionSequence`
        (:`then_0`
          (goto _label_4 :!via `Open`))
        (:`then_1`
          (`KismetSystemLibrary.Delay` (`KismetMathLibrary.RandomFloatInRange` 3.0 10.0) :!label _label_3)
          (`/Engine/EditorBlueprintResources/StandardMacros.Gate` false :!label _label_4
            (:`Exit`
              (if (`KismetMathLibrary.RandomBool`)
                (set `self.XSpeed` -10.0)
                (goto _label_3)
                (else
                  (set `self.XSpeed` 10.0)
                  (goto _label_3))))))))))

(event `self.ReceiveBeginPlay`
  (bind _xmaxdistance (`self.XMaxDistance`))
  (bind _zmaxdistance (`self.ZMaxDistance`))
  (bind (_origin _boxextent) (`KismetSystemLibrary.GetComponentBounds` (`self.PaperSprite`)))
  (bind _outactors (`GameplayStatics.GetAllActorsOfClass` "/Game/LD42/Ingredients/Board/Bp_Board.BP_Board_C"))
  (bind _output (`|GetArrayItem` _outactors))
  (set `self.XMaxDistance` (- (`/Game/LD42/Ingredients/Board/Bp_Board.XMaxDistance` _output) (.x _boxextent)))
  (set `self.ZMaxDistance` (- (`/Game/LD42/Ingredients/Board/Bp_Board.ZMaxDistance` _output) (.z _boxextent)))
  (set `self.CurrentPosition` (`KismetMathLibrary.MakeVector` (`KismetMathLibrary.RandomFloatInRange` (* _xmaxdistance -1.0) _xmaxdistance) 15.0 (`KismetMathLibrary.RandomFloatInRange` (* _zmaxdistance -1.0) _zmaxdistance)))
  (`|ExecutionSequence`
    (:`then_0`
      (goto _label_4))
    (:`then_1`
      (goto _label_2))))

(event `self.ReceiveTick`
  (params (DeltaSeconds :type "Float (single-precision)"))
  (bind _xmaxdistance (`self.XMaxDistance`))
  (bind _zmaxdistance (`self.ZMaxDistance`))
  (bind _deltatime (`self.DeltaTime`))
  (bind (_returnvalue_x _returnvalue_y _returnvalue_z) (`KismetMathLibrary.BreakVector` (- (`self.K2_GetActorLocation` (`GameplayStatics.GetPlayerPawn` 0)) (`self.K2_GetActorLocation` self))))
  (bind _returnvalue (+ (`self.CurrentPosition`) (`KismetMathLibrary.MakeVector` (* _deltatime (`self.XSpeed`)) 0.0 (* _deltatime (`self.ZSpeed`)))))
  (bind _x (.x _returnvalue))
  (bind _z (.z _returnvalue))
  (bind _returnvalue_2 (+ (.location (`self.GetTransform` self)) (0.0 5.0 0.0)))
  (set `self.DeltaTime` DeltaSeconds)
  (`|ExecutionSequence`
    (:`then_0`
      (if (`self.IsHappy`)
        _
        (elif (<= (`KismetMathLibrary.VSize` (`KismetMathLibrary.MakeVector` _returnvalue_x 0.0 _returnvalue_z)) 20.0)
          (`/Engine/EditorBlueprintResources/StandardMacros.DoOnce` false :!label _label_5
            (:`Completed`
              (`KismetSystemLibrary.RetriggerableDelay` 0.5)
              (`|ExecutionSequence`
                (:`then_0`
                  (set `self.IsHappy` true)
                  (`KismetSystemLibrary.Delay` 10.0)
                  (set `self.IsHappy` false)
                  (`PaperSpriteComponent.SetSprite` (`self.PaperSprite`) "/Game/LD42/Ingredients/Citizen/SPT_Citizen_Neutral.SPT_Citizen_Neutral"))
                (:`then_1`
                  (`PaperSpriteComponent.SetSprite` (`self.PaperSprite`) "/Game/LD42/Ingredients/Citizen/SPT_Citizen_Happy.SPT_Citizen_Happy"))
                (:`then_2`
                  (`/Engine/EditorBlueprintResources/StandardMacros.Do N` 5 :!label _label_6
                    (:`Exit`
                      (bind _returnvalue_3 (`|SpawnActorFromClass` "/Game/LD42/Ingredients/Ressource/BP_Ressources.BP_Ressources_C" (`KismetMathLibrary.MakeTransform` _returnvalue_2 (.rotation (`self.GetTransform` self)) (.scale (`self.GetTransform` self))) "Undefined" "OverrideRootScale" null null))
                      (set `/Game/LD42/Ingredients/Ressource/BP_Ressources.SpawnLocation` _returnvalue_2 _returnvalue_3)
                      (goto _label_6))))
                (:`then_3`
                  (`|ExecutionSequence` :!label _label_7
                    (:`then_0`
                      (goto _label_5 :!via `Reset`))
                    (:`then_1`
                      (goto _label_6 :!via `Reset`)))))))
          (else
            (goto _label_7)))))
    (:`then_1`
      (`self.K2_SetActorLocation` _returnvalue)
      (set `self.CurrentPosition` _returnvalue)
      (if (or (<= _x (* _xmaxdistance -1.0)) (>= _x _xmaxdistance))
        (`self.REtriggerXSpeedChange`))
      (if (or (>= _z _zmaxdistance) (<= _z (* _zmaxdistance -1.0)))
        (`self.RetriggerZSpeedChange`)))))

(fn `UserConstructionScript`)