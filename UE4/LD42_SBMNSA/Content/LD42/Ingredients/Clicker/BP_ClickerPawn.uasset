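; BP_ClickerPawn is a pawn that collects resources and opens the pause menu through cursor traces.
; On BeginPlay it enables input and shows the mouse cursor.
; Each Tick traces under the cursor, disabling collision on any BP_Ressources hit and calling HasBeenClikedOn, or creating WBP_PauseMenu for actors tagged IsPauseButton.
; No click is checked, so hovering triggers both; a note flags the pause button as needing OnClicked.
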(event `self.ReceiveBeginPlay`
  (bind _returnvalue (`GameplayStatics.GetPlayerController` 0))
  (`self.EnableInput` _returnvalue)
  (set `PlayerController.bShowMouseCursor` true _returnvalue))

(event `Key|LeftMouseButton` :consume false
  (params (Key :type "Key Structure")))

(event `self.ReceiveTick`
  (params (DeltaSeconds :type "Float (single-precision)"))
  (bind _hitresult (`PlayerController.GetHitResultUnderCursorByChannel` (`GameplayStatics.GetPlayerController` 0) "TraceTypeQuery1" true))
  (bind _asbp_ressources (cast `/Game/LD42/Ingredients/Ressource/BP_Ressources` (`.HitActor` (`GameplayStatics.BreakHitResult` _hitresult)))
    (:`then`
      (`self.SetActorEnableCollision` _asbp_ressources false)
      (`/Game/LD42/Ingredients/Ressource/BP_Ressources.HasBeenClikedOn` _asbp_ressources))
    (:`CastFailed`
      (if (`self.ActorHasTag` (`.HitActor` (`GameplayStatics.BreakHitResult` _hitresult)) "IsPauseButton")
        ;[1 1 1] Need OnClicked
        (bind _returnvalue (`|CreateWidget` "/Game/LD42/Menu/WBP_PauseMenu.WBP_PauseMenu_C"))
        (`UserWidget.AddToViewport` _returnvalue 0)))))

(fn `UserConstructionScript`)