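; BP_Ressources is a clickable resource pickup sprite that drops from a spawn point and expires unless clicked.
; On BeginPlay one timeline lerps it toward a randomly jittered X/Z target, which adds SpawnLocation twice.
; A second timeline fades the sprite from white to black, then destroys the actor.
; HasBeenClikedOn stops both timelines, preventing that destruction, and tints the sprite yellow-green.
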(event `self.ReceiveBeginPlay`
  (bind _returnvalue (`KismetMathLibrary.RandomFloatInRange` -20.0 20.0))
  (bind _spawnlocation (`self.SpawnLocation`))
  (`|ExecutionSequence`
    (:`then_0`
      (set `self.DropLocation` (+ (`self.SpawnLocation`) (`KismetMathLibrary.MakeVector` _returnvalue 0.0 _returnvalue)))
      (bind (_direction _alpha) (`Timeline|Timeline_0` :!label _label)
        (:`Update`
          (`self.K2_SetActorLocation` self (`KismetMathLibrary.VLerp` _spawnlocation (+ _spawnlocation (`self.DropLocation`)) _alpha) false false))))
    (:`then_1`
      (bind (_direction_2 _alpha_2) (`Timeline|Timeline_1` :!label _label_2)
        (:`Update`
          (`PaperSpriteComponent.SetSpriteColor` (`self.PaperSprite`) (`KismetMathLibrary.LinearColorLerp` (struct :`R` 1.0 :`G` 1.0 :`B` 1.0 :`A` 1.0) (struct) _alpha_2)))
        (:`Finished`
          (`self.K2_DestroyActor`))))))

(event `HasBeenClikedOn`
  (`|ExecutionSequence`
    (:`then_0`
      (goto _label_2 :!via `Stop`))
    (:`then_1`
      (goto _label :!via `Stop`))
    (:`then_2`
      (`PaperSpriteComponent.SetSpriteColor` (`self.PaperSprite`) (struct :`R` 0.658571 :`G` 1.0 :`A` 1.0)))))

(fn `UserConstructionScript`)