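; BP_BarkReserve displays the bark resource actors, referred to as hearts, around the dog pawn.
; On BeginPlay it attaches itself to the first BP_DogPawn at a small offset and caches its spline length.
; UpdateHeartPosition spaces the BarkRessource actors evenly along the spline.
; The first ten sit on the spline; extras form a second row, offset perpendicular to the spline direction.
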(event `self.ReceiveBeginPlay`
  (bind _outactors (`GameplayStatics.GetAllActorsOfClass` "/Game/LD42/Ingredients/Character/BP_DogPawn.BP_DogPawn_C"))
  (bind _output (`|GetArrayItem` _outactors))
  (`self.K2_AttachToActor` _output "None" "SnapToTarget" "KeepWorld" "KeepWorld")
  (`self.K2_SetActorLocation` self (+ (`self.K2_GetActorLocation` _output) (-0.5 0.0 12.0)) false false)
  (set `self.SplineLength` (`SplineComponent.GetSplineLength` (`self.Spline`))))

(event `UpdateHeartPosition`
  (bind _barkressource (`self.BarkRessource`))
  (bind _spline (`self.Spline`))
  (bind _returnvalue (`KismetArrayLibrary.Array_Length` _barkressource))
  ;[1 1 1] Set heart location on spline depending on array lenght
  (for (_array_element _array_index) _barkressource
    (bind _returnvalue_2 (> _array_index 9))
    (bind _returnvalue_3 (* (select `bool` _returnvalue_2 :`false` _array_index :`true` (- _array_index 10)) (/ (`self.SplineLength`) (`KismetMathLibrary.Conv_IntToDouble` (select `bool` _returnvalue_2 :`false` (`KismetMathLibrary.Clamp` _returnvalue 0 10) :`true` (- _returnvalue 10))))))
    (bind _returnvalue_4 (`SplineComponent.GetLocationAtDistanceAlongSpline` _spline _returnvalue_3 "World"))
    (`self.K2_SetActorLocation` _array_element (`KismetMathLibrary.SelectVector` (+ _returnvalue_4 (`KismetMathLibrary.GreaterGreater_VectorRotator` (* (`SplineComponent.GetDirectionAtDistanceAlongSpline` _spline _returnvalue_3 "World") 8.0) (struct :`Pitch` 90.0))) _returnvalue_4 _returnvalue_2) false false)))

(fn `UserConstructionScript`)