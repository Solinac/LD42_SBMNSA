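; BP_Outbreak spreads corruption across the board's tiles from an initial set of corrupted tiles.
; On BeginPlay it corrupts those tiles, then starts a looping timer that runs Corruption.
; Each tick gathers neutral neighbors of all corrupted tiles and corrupts a random one, which joins the spreading set.
; Candidates may repeat, favoring tiles with several corrupted neighbors, and the random index never selects the last of multiple entries.
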(event `self.ReceiveBeginPlay`
  (`|ExecutionSequence`
    (:`then_0`
      ;[1 1 1] Corrupt initial tiles
      (for _array_element (`self.CorruptedTiles`)
        (`self.CorruptTile` _array_element)))
    (:`then_1`
      ;[1 1 1] Corruption cycle
      (`KismetSystemLibrary.K2_SetTimerDelegate` (delegate `CustomEvent_0`) (`self.NewCorruptionTimer`) true))))

(event `CustomEvent_0`
  ;[1 1 1] Corruption cycle
  (`self.Corruption`))

(fn `Corruption`
  (bind _adjacentneutraltiles (`self.AdjacentNeutralTiles`))
  (`KismetArrayLibrary.Array_Clear` (`self.AdjacentNeutralTiles`))
  (for _array_element (`self.CorruptedTiles`)
    (bind _adjacenttiles (`/Game/LD42/Ingredients/Board/Bp_Board.GetAdjacentTiles` (`/Game/LD42/Ingredients/BP_FunctionLibrary.GetBoard`) (`/Game/LD42/Ingredients/Board/BP_Tile.Coordinates` _array_element)))
    (for _array_element_2 _adjacenttiles
      (if (`|EnumEquality` "NewEnumerator0" (`/Game/LD42/Ingredients/Board/BP_Tile.TileState` _array_element_2))
        (`KismetArrayLibrary.Array_Add` (`self.AdjacentNeutralTiles`) _array_element_2))))
  (if (!= (`KismetArrayLibrary.Array_Length` (`self.AdjacentNeutralTiles`)) 0)
    (`self.CorruptTile` (`|GetArrayItem` _adjacentneutraltiles (`KismetMathLibrary.RandomInteger` (- (`KismetArrayLibrary.Array_Length` _adjacentneutraltiles) 1))))))

(fn `CorruptTile`
  (params (Tile :type "/Game/LD42/Ingredients/Board/BP_Tile Object Reference"))
  (`|ExecutionSequence`
    (:`then_0`
      (`/Game/LD42/Ingredients/Board/BP_Tile.ChangeTileState` Tile "NewEnumerator1"))
    (:`then_1`
      (`KismetArrayLibrary.Array_AddUnique` (`self.CorruptedTiles`) Tile))))

(fn `UserConstructionScript`)